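; Goblin enemy that walks to a tower and attacks it.
; It picks a random BP_TowerBase at BeginPlay and switches to the closest one whenever that target is no longer valid.
; Tick issues AIMoveTo toward the tower; once in close range, it sets IsAttacking and calls the attack event.
; If BoxAttackTrigger overlaps the tower at that moment, it damages the tower's BPHealthComponent.
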(event EventBeginPlay
  (|CallParentFunction)
  (bind _tower (CallFunction|GetRandomTower))
  (Variables|Default|SetTower _tower))

(event EventTick
  (params (DeltaSeconds :type Float%20%28single-precision%29))
  (Utilities|IsValid (Variables|Default|GetTower)
    (:Is%20Valid
      _)
    (:Is%20Not%20Valid
      (bind _tower (CallFunction|GetClosestTower))
      (Variables|Default|SetTower _tower)))
  (AI|AIMoveTo self "200.000000,200.000000,50.000000" (Variables|Default|GetTower) 5.0 false
    (:then
      (if (< (Transformation|GetDistanceTo (Variables|Default|GetTower)) 1.2e+02)
        (if (not (Variables|Default|GetIs%20Attacking))
          (Variables|Default|SetIs%20Attacking true)
          (Default|CallOnAttack)
          (if (Collision|IsOverlappingActor (Variables|Default|GetBoxAttackTrigger) (Variables|Default|GetTower) :!class /Script/Engine.PrimitiveComponent)
            (Default|Damage (Variables|/Game/Projet/Blueprints/Tower/BP_TowerBase.BP_TowerBase_C|GetBP_HealthComponent (Variables|Default|GetTower)) 1e+01)))))))

(fn ConstructionScript)

(fn GetClosestTower
  (bind _outactors (Actor|GetAllActorsOfClass "/Game/Projet/Blueprints/Tower/BP_TowerBase.BP_TowerBase_C"))
  (for _array_element _outactors
    (if (< (Transformation|GetDistanceTo _array_element) (LocalVariables|GetDistance))
      (LocalVariables|SetDistance (Transformation|GetDistanceTo _array_element))
      (LocalVariables|SetTarget%20Tower _array_element)))
  (return (LocalVariables|GetTarget%20Tower)))

(fn GetRandomTower
  (bind _outactors (Actor|GetAllActorsOfClass "/Game/Projet/Blueprints/Tower/BP_TowerBase.BP_TowerBase_C"))
  (return (.OutItem (Utilities|Array|Random _outactors))))