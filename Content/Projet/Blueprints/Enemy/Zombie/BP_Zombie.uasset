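; Zombie enemy Blueprint that walks toward the nearest tower.
; On BeginPlay it sets its walk speed, caches all BP_TowerBase actors and picks the closest, keeping a running Distance that is never reset.
; Tick reissues AI MoveTo every frame and searches the cached list again when the target becomes invalid.
; Health component changes update the health bar widget and briefly raise an IsHit flag.
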(event OnHealthChange(BP_HealthComponent)
  (params (Health :type Float%20%28double-precision%29) (Max%20Health :type Float%20%28double-precision%29))
  (bind _aswb_health_bar (Utilities|Casting|CastToWB_HealthBar (UserInterface|GetUserWidgetObject (Variables|Default|GetHealthBar))))
  (Default|SetRemainingHealth _aswb_health_bar Health Max%20Health)
  (Variables|Default|SetIsHit true)
  (Utilities|FlowControl|Delay 0.1)
  (Variables|Default|SetIsHit false))

(event EventBeginPlay
  (|CallParentFunction)
  (Variables|/Script/Engine.CharacterMovementComponent|SetMaxWalkSpeed (Variables|Character|GetCharacterMovement) 125.0)
  (bind _outactors (Actor|GetAllActorsOfClass "/Game/Projet/Blueprints/Tower/BP_TowerBase.BP_TowerBase_C"))
  (Variables|Default|SetTowers _outactors)
  (CallFunction|FindTarget))

(event Collision|EventActorBeginOverlap
  (params (OtherActor :type Actor%20Object%20Reference)))

(event EventTick
  (params (DeltaSeconds :type Float%20%28single-precision%29))
  (Utilities|IsValid (Variables|Default|GetTarget)
    (:Is%20Valid
      _)
    (:Is%20Not%20Valid
      (CallFunction|FindTarget)))
  (AI|AIMoveTo self "0, 0, 0" (Variables|Default|GetTarget) 5.0 false))

(fn ConstructionScript
  (|CallParentFunction))

(fn FindTarget
  (for _array_element (Variables|Default|GetTowers)
    (Utilities|IsValid _array_element
      (:Is%20Valid
        (bind _returnvalue (CallFunction|ComputeDistance _array_element))
        (if (< _returnvalue (Variables|Default|GetDistance))
          (Variables|Default|SetDistance _returnvalue)
          (Variables|Default|SetTarget _array_element))))))

(fn ComputeDistance
  (params (Tower :type BP%20Tower%20Base%20Object%20Reference))
  (return (Math|Vector|Distance(Vector) (Transformation|GetActorLocation Tower) (Transformation|GetActorLocation))))