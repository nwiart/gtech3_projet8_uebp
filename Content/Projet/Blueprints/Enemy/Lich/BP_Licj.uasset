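; Lich enemy that walks to a random tower from the game instance and attacks it, switching to the closest when that becomes invalid.
; Tick drives AIMoveTo; in range, a DoOnce rolls melee damage, projectile or beam attack, with melee shortening the acceptance radius.
; Delays time each hit to animation switches, and the roll resets only when movement fails out of range.
; Death spawns particles, then destroys the actor after a delay.
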(event OnDeath(BP_HealthComponent)
  (bind _self self)
  (bind _returnvalue (Transformation|GetActorTransform _self))
  (Game|SpawnActorfromClass "/Game/Projet/Blueprints/Enemy/Lich/BP_DeadParticles.BP_DeadParticles_C" (Math|Transform|MakeTransform (.location _returnvalue) (.rotation _returnvalue) "1.000000,1.000000,1.000000") "Undefined" "MultiplyWithRoot" 0 0)
  (Utilities|FlowControl|Delay 3.0)
  (Actor|DestroyActor))

(event EventBeginPlay
  (|CallParentFunction)
  (bind _tower (CallFunction|GetRandomTower))
  (Variables|Default|SetTower _tower)
  (Variables|Default|SetAcceptanceRadius 6e+02))

(event Collision|EventActorBeginOverlap
  (params (OtherActor :type Actor%20Object%20Reference)))

(event EventTick
  (params (DeltaSeconds :type Float%20%28single-precision%29))
  (Utilities|IsValid (Variables|Default|GetTower)
    (:Is%20Valid
      (if (Variables|Default|GetHasFinishedSpawn)
        (if (== (Variables|Default|GetAttackType) 1)
          (Variables|Default|SetAcceptanceRadius 1.5e+02)
          (else
            (Variables|Default|SetAcceptanceRadius 5e+02)))
        (AI|AIMoveTo self "200.000000,200.000000,50.000000" (Variables|Default|GetTower) (Variables|Default|GetAcceptanceRadius) false
          (:then
            (if (not (Variables|Default|GetIs%20Attacking))
              (if (<= (Transformation|GetDistanceTo (Variables|Default|GetTower)) (+ (Variables|Default|GetAcceptanceRadius) 5e+01))
                (Variables|Default|SetIs%20Attacking true)
                (Utilities|FlowControl|DoOnce false :!label _label
                  (:Completed
                    (Variables|Default|SetAttackType (Math|Random|RandomIntegerinRange 1 3)))))
              (elif (not (Variables|Default|GetIsDoingAnAttack))
                (Variables|Default|SetIsDoingAnAttack true)
                (switch int (Variables|Default|GetAttackType)
                  (:1
                    (Variables|Default|SetAttackAnimationSwitch true)
                    (bind _output_get (Variables|Default|SetNormalAttackType (Math|Random|RandomIntegerinRange 0 1)))
                    (switch int _output_get
                      (:0
                        (Utilities|FlowControl|Delay 0.54))
                      (:1
                        (Utilities|FlowControl|Delay 0.84)))
                    (CallFunction|CloseAttack)
                    (switch int 0
                      (:0
                        (Utilities|FlowControl|Delay 1.13))
                      (:1
                        (Utilities|FlowControl|Delay 0.99))))
                  (:2
                    (Variables|Default|SetAttackAnimationSwitch true)
                    (Utilities|FlowControl|Delay 1.15)
                    (CallFunction|TrowProjectile)
                    (Utilities|FlowControl|Delay 1.05))
                  (:3
                    (Variables|Default|SetAttackAnimationSwitch true)
                    (Utilities|FlowControl|Delay 0.48)
                    (CallFunction|TheCall)
                    (Utilities|FlowControl|Delay 1.85)))
                (Variables|Default|SetAttackAnimationSwitch false)
                (Variables|Default|SetIsDoingAnAttack false))))
          (:OnFail
            (if (not (< (Transformation|GetDistanceTo (Variables|Default|GetTower)) 5.2e+02))
              (Variables|Default|SetAttackType 0)
              (Variables|Default|SetIs%20Attacking false)
              (goto _label Reset))))))
    (:Is%20Not%20Valid
      (bind _tower (CallFunction|GetClosestTower))
      (Variables|Default|SetTower _tower))))

(fn ConstructionScript
  (|CallParentFunction))

(fn GetClosestTower
  (bind _asbp_tower_game_instance (Utilities|Casting|CastToBP_TowerGameInstance (Game|GetGameInstance)))
  (bind _result (Utilities|Set|ToArray (Variables|/Game/Projet/Blueprints/BP_TowerGameInstance.BP_TowerGameInstance_C|GetTowers _asbp_tower_game_instance)))
  (for _array_element _result
    (if (< (Transformation|GetDistanceTo _array_element) (LocalVariables|GetDistance))
      (LocalVariables|SetDistance (Transformation|GetDistanceTo _array_element))
      (LocalVariables|SetTargetTower _array_element)))
  (return (LocalVariables|GetTargetTower)))

(fn GetRandomTower
  (bind _asbp_tower_game_instance (Utilities|Casting|CastToBP_TowerGameInstance (Game|GetGameInstance)))
  (bind _result (Utilities|Set|ToArray (Variables|/Game/Projet/Blueprints/BP_TowerGameInstance.BP_TowerGameInstance_C|GetTowers _asbp_tower_game_instance)))
  (return (.OutItem (Utilities|Array|Random _result))))

(fn CloseAttack
  (bind _tower (Variables|Default|GetTower))
  (bind _bp_healthcomponent (Variables|/Game/Projet/Blueprints/Tower/BP_TowerBase.BP_TowerBase_C|GetBP_HealthComponent _tower))
  (Utilities|IsValid _tower
    (:Is%20Valid
      (Utilities|IsValid _bp_healthcomponent
        (:Is%20Valid
          (Default|Damage _bp_healthcomponent 15.0))))))

(fn TrowProjectile
  (bind _firepoint (Variables|Default|GetFirePoint))
  (bind _returnvalue (Transformation|GetWorldTransform _firepoint))
  (Game|SpawnActorfromClass "/Game/Projet/Blueprints/Enemy/Lich/BP_LichProjectile.BP_LichProjectile_C" (Math|Transform|MakeTransform (.location _returnvalue) (.rotation _returnvalue) "1.000000,1.000000,1.000000") "Undefined" "MultiplyWithRoot" self 0))

(fn TheCall
  (bind _tower (Variables|Default|GetTower))
  (bind _tower_2 (Variables|Default|GetTower))
  (bind _returnvalue (Transformation|GetActorTransform _tower))
  (Utilities|IsValid _tower
    (:Is%20Valid
      (bind _returnvalue_2 (Game|SpawnActorfromClass "/Game/Projet/Blueprints/Enemy/Lich/BP_Beam.BP_Beam_C" (Math|Transform|MakeTransform (.location _returnvalue) (.rotation _returnvalue) "1.000000,1.000000,1.000000") "Undefined" "MultiplyWithRoot" 0 0))
      (Utilities|IsValid _tower_2
        (:Is%20Valid
          (Default|InitDamage _returnvalue_2 _tower_2))))))