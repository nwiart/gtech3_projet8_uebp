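; Projectile for the Lich enemy that damages what it hits through the health component.
; The Sphere's hit event applies fixed damage to any actor with a BP_HealthComponent and spawns a BP_HitExplode at the projectile's transform.
; The projectile destroys itself on hitting any valid actor, so the explosion appears only on damageable targets.
; An unconnected loop for toggling the Sphere's ignored actors never runs.
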(event OnComponentHit(Sphere)
  (params (HitComponent :type Primitive%20Component%20Object%20Reference) (OtherActor :type Actor%20Object%20Reference) (OtherComp :type Primitive%20Component%20Object%20Reference) (NormalImpulse :type Vector :default "0, 0, 0") (Hit :type Hit%20Result%20Structure%20%28by%20ref%29))
  (bind _returnvalue (Actor|GetComponentbyClass OtherActor "/Game/Projet/Blueprints/BP_HealthComponent.BP_HealthComponent_C"))
  (bind _self self)
  (bind _returnvalue_2 (Transformation|GetActorTransform _self))
  (Utilities|IsValid OtherActor
    (:Is%20Valid
      (Utilities|IsValid _returnvalue
        (:Is%20Valid
          (Default|Damage _returnvalue 1e+01)
          (Game|SpawnActorfromClass "/Game/Projet/Blueprints/Enemy/Lich/BP_HitExplode.BP_HitExplode_C" (Math|Transform|MakeTransform (.location _returnvalue_2) (.rotation _returnvalue_2) "1.000000,1.000000,1.000000") "AlwaysSpawn" "MultiplyWithRoot" 0 0))
        (:Is%20Not%20Valid
          _))
      (Actor|DestroyActor))))

(event EventBeginPlay)

(event Collision|EventActorBeginOverlap
  (params (OtherActor :type Actor%20Object%20Reference)))

(event EventTick
  (params (DeltaSeconds :type Float%20%28single-precision%29)))

(fn ConstructionScript)