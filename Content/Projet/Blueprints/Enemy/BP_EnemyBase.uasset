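; Base enemy Blueprint that links a health component to a health bar widget and handles death.
; On BeginPlay it caches the WB_HealthBar widget and shows the initial health, then refreshes the bar whenever the component reports a health change.
; On death it flags itself dead, hides the bar, disables capsule collision and actor tick, and unpossesses its controller to stop movement.
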(event OnHealthChange(BP_HealthComponent)
  (params (Health :type Float%20%28double-precision%29) (Max%20Health :type Float%20%28double-precision%29))
  ;[1 1 1] Health component implementation
  (bind _aswb_health_bar (Utilities|Casting|CastToWB_HealthBar (UserInterface|GetUserWidgetObject (Variables|Default|GetHealthBar))))
  (Default|SetRemainingHealth _aswb_health_bar Health Max%20Health))

(event OnDeath(BP_HealthComponent)
  ;[1 1 1] Health component implementation
  (Variables|Default|SetIs%20Dead true)
  (Development|SetHiddeninGame (Variables|Default|GetHealthBar) true false)
  (Collision|SetCollisionEnabled (Variables|Collision|GetCapsuleComponent) "NoCollision")
  ;;[1 1 1] Disable tick and controller, so that all movement becomes impossible
  (Actor|Tick|SetActorTickEnabled false)
  (Pawn|UnPossess (Pawn|GetController)))

(event EventBeginPlay
  (bind _bp_healthcomponent (Variables|Default|GetBP_HealthComponent))
  ;[1 1 1] Initial health update
  (bind _aswb_health_bar (Utilities|Casting|CastToWB_HealthBar (UserInterface|GetUserWidgetObject (Variables|Default|GetHealthBar))))
  (Variables|Default|SetHealthUI _aswb_health_bar)
  (Default|SetRemainingHealth _aswb_health_bar (Variables|/Game/Projet/Blueprints/BP_HealthComponent.BP_HealthComponent_C|GetHealth _bp_healthcomponent) (Variables|/Game/Projet/Blueprints/BP_HealthComponent.BP_HealthComponent_C|GetMax%20Health _bp_healthcomponent)))

(fn ConstructionScript)