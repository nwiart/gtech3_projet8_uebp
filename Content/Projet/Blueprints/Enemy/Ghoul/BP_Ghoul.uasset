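; Ghoul enemy Blueprint that chases the player and flags when it is attacking or hit.
; A looping one-second timer issues AI MoveTo toward the player pawn when beyond attack range, clearing IsAttacking and setting it on arrival.
; Health component changes raise IsHit, which clears after a short delay.
; The file only sets these flags and applies no damage itself.
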(event OnHealthChange(BP_HealthComponent)
  (params (Health :type Float%20%28double-precision%29) (Max%20Health :type Float%20%28double-precision%29))
  (Variables|Default|Setis%20Hit true)
  (Utilities|FlowControl|Delay 1.0)
  (Variables|Default|Setis%20Hit false))

(event Custom|Chase%20Target
  (if (> (Math|Vector|Distance(Vector) (Transformation|GetActorLocation) (Transformation|GetActorLocation (Variables|Default|GetTarget))) 1.8e+02)
    (Variables|Default|Setis%20Attacking false)
    (AI|AIMoveTo self "0.000000,0.000000,0.000000" (Game|Player|GetPlayerPawn 0) 1.1e+02 false
      (:OnSuccess
        (Variables|Default|Setis%20Attacking true)))))

(event EventBeginPlay
  (|CallParentFunction)
  (Utilities|Time|SetTimerbyEvent (delegate Custom|Chase%20Target) 1.0 true)
  (Variables|Default|SetTarget (Game|Player|GetPlayerPawn 0)))

(fn ConstructionScript
  (|CallParentFunction))