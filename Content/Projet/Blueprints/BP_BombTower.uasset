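; BP_BombTower is a tower actor that periodically launches bombs at a nearby player.
; A looping timer started on BeginPlay checks the first player pawn's distance every second.
; Within range, it spawns a BP_Bomb at its own location and applies a Force-scaled physics impulse to the bomb's mesh toward the player.
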(event Custom|Shooting
  (bind _returnvalue (Transformation|GetActorLocation))
  (if (<= (Transformation|GetDistanceTo (Game|Player|GetPlayerPawn 0) 0) 2e+02)
    (bind _returnvalue_2 (Game|SpawnActorfromClass "/Game/Projet/Blueprints/BP_Bomb.BP_Bomb_C" (Math|Conversions|ToTransform(Vector) _returnvalue) "Undefined" "MultiplyWithRoot" 0 0))
    (Physics|AddImpulse (Variables|/Game/Projet/Blueprints/BP_Bomb.BP_Bomb_C|GetStaticMesh _returnvalue_2) (* (Math|Vector|GetUnitDirection(Vector) _returnvalue (Transformation|GetActorLocation (Game|Player|GetPlayerPawn 0))) (Variables|Default|GetForce)) "None" false)))

(event EventBeginPlay
  (bind _returnvalue (Utilities|Time|SetTimerbyEvent (delegate Custom|Shooting) 1.0 true))
  (Variables|Default|SetTimer _returnvalue))

(fn ConstructionScript)