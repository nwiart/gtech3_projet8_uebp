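; Actor health component that tracks Health against MaxHealth and exposes Heal and Damage functions.
; Heal adds to Health capped at MaxHealth, while Damage subtracts down to zero and is ignored once Health is already depleted.
; Both broadcast OnHealthChange with current and max values, and Damage fires OnDeath when Health reaches zero.
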(fn Heal
  (params (Amount :type Float%20%28double-precision%29))
  (bind _max_health (Variables|Default|GetMax%20Health))
  (bind _output_get (Variables|Default|SetHealth (Math|Float|Min(Float) (+ Amount (Variables|Default|GetHealth)) _max_health)))
  (Default|CallOnHealthChange _output_get _max_health))

(fn Damage
  (params (Amount :type Float%20%28double-precision%29))
  (if (> (Variables|Default|GetHealth) 0.0)
    (bind _output_get (Variables|Default|SetHealth (Math|Float|Max(Float) (- (Variables|Default|GetHealth) Amount) 0.0)))
    (Default|CallOnHealthChange _output_get (Variables|Default|GetMax%20Health))
    (if (== _output_get 0.0)
      (Default|CallOnDeath))))