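; BP_TowerRadial is a tower that pushes back targets with a radial impulse.
; On BeginPlay it runs the parent setup and starts a looping Shoot timer at the ShootTimer interval.
; When the TargetCharacters set is not empty, Shoot spawns a BP_RadialPush actor at the ShootSource location and fires the RadialForce component's impulse.
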(event Custom|Shoot
  (if (Utilities|Set|IsNotEmpty (Variables|Default|GetTarget%20Characters))
    (Game|SpawnActorfromClass "/Game/Projet/Blueprints/Tower/BP_RadialPush.BP_RadialPush_C" (Math|Conversions|ToTransform(Vector) (Transformation|GetWorldLocation (Variables|Default|GetShootSource))) "Undefined" "MultiplyWithRoot" 0 0)
    (Class|RadialForceComponent|FireImpulse (Variables|Default|GetRadialForce))))

(event EventBeginPlay
  (|CallParentFunction)
  (Utilities|Time|SetTimerbyEvent (delegate Custom|Shoot) (Variables|Default|GetShoot%20Timer) true))

(fn ConstructionScript)