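; BP_TowerVortex is a tower that periodically fires vortex balls at targets and takes damage from first-person projectiles.
; A looping timer calls Shooting, which, when TargetCharacters is not empty, spawns a BP_VortexBall and sets its physics velocity toward a random in-range target.
; Random target picks are not cached, so the ball's facing and velocity can point at different targets.
; Projectile hits on the Cube apply fixed damage to BPHealthComponent.
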(event OnComponentHit(Cube)
  (params (HitComponent :type Primitive%20Component%20Object%20Reference) (OtherActor :type Actor%20Object%20Reference) (OtherComp :type Primitive%20Component%20Object%20Reference) (NormalImpulse :type Vector :default "0, 0, 0") (Hit :type Hit%20Result%20Structure%20%28by%20ref%29))
  (Utilities|Casting|CastToBP_FirstPersonProjectile OtherActor)
  (Default|Damage (Variables|Default|GetBP_HealthComponent) 1e+01))

(event Custom|ShootingEvent
  (CallFunction|Shooting))

(event EventBeginPlay
  (|CallParentFunction)
  (Utilities|Time|SetTimerbyEvent (delegate Custom|ShootingEvent) (Variables|Default|GetShootingDelay) true))

(fn ConstructionScript)

(fn Shooting
  (bind _returnvalue (Transformation|GetActorLocation))
  (bind _character (CallFunction|PickRandomTargetinRange))
  (bind _spawnoffset (Variables|Default|GetSpawnOffset))
  (bind _returnvalue_2 (Transformation|GetActorLocation _character))
  (bind _returnvalue_3 (+ _returnvalue _spawnoffset))
  (bind _returnvalue_4 (Math|Vector|GetUnitDirection(Vector) _returnvalue_3 _returnvalue_2))
  (if (Utilities|Set|IsNotEmpty (Variables|Default|GetTarget%20Characters))
    (bind _returnvalue_5 (Game|SpawnActorfromClass "/Game/Projet/Blueprints/Tower/BP_VortexBall.BP_VortexBall_C" (Math|Transform|MakeTransform _returnvalue_3 (Math|Rotator|MakeRotfromXY _returnvalue_4 _returnvalue_4) "1.000000,1.000000,1.000000") "Undefined" "MultiplyWithRoot" 0 0))
    ;[1 1 1] Apply force to our projectile
    (Physics|SetPhysicsLinearVelocity (Variables|/Game/Projet/Blueprints/Tower/BP_VortexBall.BP_VortexBall_C|GetCollisionComponent _returnvalue_5) (* (Math|Vector|GetUnitDirection(Vector) (Transformation|GetWorldLocation (Variables|Default|GetSpawnPoint)) (Transformation|GetActorLocation (CallFunction|PickRandomTargetinRange))) 5e+02) false "None")))