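; BPC_Vortex is a component, filed with the tower Blueprints, that creates a vortex at its owner's position.
; INit stores a RadialForce reference supplied from outside.
; ActivateVortex plays a sound, spawns a BPC_BlackHole actor at the owner's location and rotation, and sets a flag.
; While that flag is set, Tick fires the radial impulse every frame, and nothing here clears it.
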(event EventBeginPlay
  (Variables|Default|SetOwner (Components|GetOwner)))

(event EventTick
  (params (DeltaSeconds :type Float%20%28single-precision%29))
  (if (Variables|Default|GetVortexActivated)
    (Class|RadialForceComponent|FireImpulse (Variables|Default|GetRadialForce))))

(fn ActivateVortex
  (bind _owner (Variables|Default|GetOwner))
  (bind _returnvalue (Transformation|GetActorTransform _owner))
  (Audio|PlaySoundatLocation 0 (Transformation|GetActorLocation (Variables|Default|GetOwner)) "0, 0, 0" 1.0 1.0 0.0 0 0 0 0)
  (Game|SpawnActorfromClass "/Game/Projet/Blueprints/Tower/BPC_BlackHole.BPC_BlackHole_C" (Math|Transform|MakeTransform (.location _returnvalue) (.rotation _returnvalue) "1.000000,1.000000,1.000000") "Undefined" "MultiplyWithRoot" 0 0)
  (Variables|Default|SetVortexActivated true))

(fn INit
  (params (RadialForce :type Radial%20Force%20Component%20Object%20Reference))
  (Variables|Default|SetRadialForce RadialForce))