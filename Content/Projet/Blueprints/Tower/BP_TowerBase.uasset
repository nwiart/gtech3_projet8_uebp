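; Base tower actor with a health bar and optional detection of characters in range for defense.
; The health component pushes changes to the health bar widget and destroys the actor on death.
; The construction script sizes the detection sphere when the tower can defend, and otherwise disables its collision.
; Sphere overlaps keep a set of target characters, from which a helper function picks one at random.
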(event OnHealthChange(BP_HealthComponent)
  (params (Health :type Float%20%28double-precision%29) (Max%20Health :type Float%20%28double-precision%29))
  ;[1 1 1] Health component integration
  (Default|SetRemainingHealth (Variables|Default|GetHealth%20Bar%20Widget) Health Max%20Health))

(event OnDeath(BP_HealthComponent)
  ;[1 1 1] Health component integration
  (Actor|DestroyActor))

(event OnComponentBeginOverlap(DetectRangeCollider)
  (params (OverlappedComponent :type Primitive%20Component%20Object%20Reference) (OtherActor :type Actor%20Object%20Reference) (OtherComp :type Primitive%20Component%20Object%20Reference) (OtherBodyIndex :type Integer) (bFromSweep :type Boolean) (SweepResult :type Hit%20Result%20Structure%20%28by%20ref%29))
  ;[1 1 1] Character detection
  (bind _ascharacter (Utilities|Casting|CastToCharacter OtherActor))
  (Utilities|Set|Add (Variables|Default|GetTarget%20Characters) _ascharacter))

(event OnComponentEndOverlap(DetectRangeCollider)
  (params (OverlappedComponent :type Primitive%20Component%20Object%20Reference) (OtherActor :type Actor%20Object%20Reference) (OtherComp :type Primitive%20Component%20Object%20Reference) (OtherBodyIndex :type Integer))
  ;[1 1 1] Character detection
  (bind _ascharacter (Utilities|Casting|CastToCharacter OtherActor))
  (Utilities|Set|Remove (Variables|Default|GetTarget%20Characters) _ascharacter))

(event EventBeginPlay
  (bind _bp_healthcomponent (Variables|Default|GetBP_HealthComponent))
  ;[1 1 1] Initial health update
  (bind _aswb_health_bar (Utilities|Casting|CastToWB_HealthBar (UserInterface|GetUserWidgetObject (Variables|Default|GetHealthBar))))
  (bind _output_get (Variables|Default|SetHealth%20Bar%20Widget _aswb_health_bar))
  (Default|SetRemainingHealth _output_get (Variables|/Game/Projet/Blueprints/BP_HealthComponent.BP_HealthComponent_C|GetHealth _bp_healthcomponent) (Variables|/Game/Projet/Blueprints/BP_HealthComponent.BP_HealthComponent_C|GetMax%20Health _bp_healthcomponent)))

(fn ConstructionScript
  (if (Variables|Default|GetCan%20Defend)
    (Components|Sphere|SetSphereRadius (Variables|Default|GetDetectRangeCollider) (Variables|Default|GetDetect%20Range) true)
    (Collision|SetCollisionEnabled (Variables|Default|GetDetectRangeCollider) "QueryOnly")
    (else
      (Collision|SetCollisionEnabled (Variables|Default|GetDetectRangeCollider) "NoCollision"))))

(fn PickRandomTargetinRange
  (bind _target_characters (Variables|Default|GetTarget%20Characters))
  (bind _result (Utilities|Set|ToArray _target_characters))
  (return (Utilities|Array|Get(acopy) _result (Math|Random|RandomInteger (Utilities|Set|Length _target_characters)))))