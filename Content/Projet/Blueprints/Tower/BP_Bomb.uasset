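; BP_Bomb is a timed bomb that explodes after a short fuse and then destroys itself.
; The fuse is a Delay driven from Event Tick rather than BeginPlay.
; When it completes, the bomb spawns BP_BombExplosion at its mesh, applies full, non-falloff radial damage that ignores itself and the first player's character, and fires a RadialForce impulse.
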(event EventTick
  (params (DeltaSeconds :type Float%20%28single-precision%29))
  (Utilities|FlowControl|Delay 3.0)
  (Game|SpawnActorfromClass "/Game/Projet/Blueprints/Tower/BP_BombExplosion.BP_BombExplosion_C" (Math|Conversions|ToTransform(Vector) (Transformation|GetWorldLocation (Variables|Default|GetStaticMesh))) "Undefined" "MultiplyWithRoot" 0 0)
  (Game|Damage|ApplyRadialDamage 5e+01 (Transformation|GetActorLocation) 5e+02 0 (Utilities|Array|MakeArray self (Game|GetPlayerCharacter 0)) self 0 true "ECC_Visibility")
  (Class|RadialForceComponent|FireImpulse (Variables|Default|GetRadialForce))
  (Actor|DestroyActor))

(event EventBeginPlay)

(fn ConstructionScript)