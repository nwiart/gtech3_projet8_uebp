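; BP_Tower1 is a tower that periodically fires projectiles at targets in range.
; On BeginPlay it runs the parent logic, then starts a looping timer that calls Shoot at the ShootTimer interval.
; When TargetCharacters is not empty, Shoot spawns ProjectileClass at ShootSource and casts it to BP_TowerProjectile.
; It launches the projectile by setting its sphere's physics velocity toward a randomly picked target in range.
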(event Custom|Shoot
  (bind _shootsource (Variables|Default|GetShootSource))
  (if (Utilities|Set|IsNotEmpty (Variables|Default|GetTarget%20Characters))
    (bind _returnvalue (Game|SpawnActorfromClass (Variables|Default|GetProjectile%20Class) (Math|Transform|MakeTransform (Transformation|GetWorldLocation _shootsource) (Transformation|GetWorldRotation _shootsource) "1.000000,1.000000,1.000000") "Undefined" "MultiplyWithRoot" 0 0))
    ;[1 1 1] Apply force to our projectile
    (bind _asbp_tower_projectile (Utilities|Casting|CastToBP_TowerProjectile _returnvalue))
    (Physics|SetPhysicsLinearVelocity (Variables|/Game/Projet/Blueprints/Tower/BP_TowerProjectile.BP_TowerProjectile_C|GetSphere _asbp_tower_projectile) (* (Math|Vector|GetUnitDirection(Vector) (Transformation|GetWorldLocation (Variables|Default|GetShootSource)) (Transformation|GetActorLocation (CallFunction|PickRandomTargetinRange))) 3e+03) false "None")))

(event EventBeginPlay
  (|CallParentFunction)
  (Utilities|Time|SetTimerbyEvent (delegate Custom|Shoot) (Variables|Default|GetShoot%20Timer) true))

(fn ConstructionScript)