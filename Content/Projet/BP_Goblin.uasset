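; BP_Goblin is an enemy character that chases the player and has a floating health bar.
; Every tick it issues an AI MoveTo toward the player pawn.
; Its health component drives the widget-based health bar on start and on every change.
; On death it flags itself dead, hides the bar, disables capsule collision, stops ticking and unpossesses its controller to halt movement.
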(event OnHealthChange(BP_HealthComponent)
  (params (Health :type Float%20%28double-precision%29) (Max%20Health :type Float%20%28double-precision%29))
  ;[1 1 1] Health component implementation
  (bind _aswb_health_bar (Utilities|Casting|CastToWB_HealthBar (UserInterface|GetUserWidgetObject (Variables|Default|GetHealthBar))))
  (Default|SetRemainingHealth _aswb_health_bar Health Max%20Health))

(event OnDeath(BP_HealthComponent)
  ;[1 1 1] Health component implementation
  (Variables|Default|SetIs%20Dead true)
  (Development|SetHiddeninGame (Variables|Default|GetHealthBar) true false)
  (Collision|SetCollisionEnabled (Variables|Collision|GetCapsuleComponent) "NoCollision")
  ;;[1 1 1] Disable tick and controller, so that all movement becomes impossible
  (Actor|Tick|SetActorTickEnabled false)
  (Pawn|UnPossess (Pawn|GetController)))

(event EventBeginPlay
  (bind _bp_healthcomponent (Variables|Default|GetBP_HealthComponent))
  (bind _aswb_health_bar (Utilities|Casting|CastToWB_HealthBar (UserInterface|GetUserWidgetObject (Variables|Default|GetHealthBar))))
  (Default|SetRemainingHealth _aswb_health_bar (Variables|/Game/Projet/Blueprints/BP_HealthComponent.BP_HealthComponent_C|GetHealth _bp_healthcomponent) (Variables|/Game/Projet/Blueprints/BP_HealthComponent.BP_HealthComponent_C|GetMax%20Health _bp_healthcomponent)))

(event EventTick
  (params (DeltaSeconds :type Float%20%28single-precision%29))
  (AI|AIMoveTo self "200.000000,200.000000,50.000000" (Game|Player|GetPlayerPawn 0) 5.0 false))

(fn ConstructionScript)