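; Inventory component that tracks ammo for a rifle, a rocket weapon and a laser weapon.
; BeginPlay seeds the counts and fills the AmmoMags array with one slot per weapon.
; ReloadRifle moves rounds from the reserve into the magazine, without capping it when the reserve is under 20, then UpdateAmmoMags copies the counts into the array.
; RefillAmmo overwrites the rifle reserve with a passed-in value.
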(event EventBeginPlay
  (bind _ammomags (Variables|Default|GetAmmoMags))
  (Variables|Default|SetRifleTotalAmmo 240)
  (Variables|Default|SetRifleCurrentAmmo 20)
  (Variables|Default|SetRIfleMaxAmmo 20)
  (Variables|Default|SetRocketAmount 2)
  (Variables|Default|SetLaserAmount 50)
  (Utilities|Array|Add _ammomags (Variables|Default|GetRifleCurrentAmmo))
  (Utilities|Array|Add _ammomags (Variables|Default|GetRocketAmount))
  (Utilities|Array|Add _ammomags (Variables|Default|GetLaserAmount)))

(event EventTick
  (params (DeltaSeconds :type Float%20%28single-precision%29)))

(fn ReloadRifle
  (bind _ammomags (Variables|Default|GetAmmoMags))
  (bind _output (Utilities|Array|Get(acopy) _ammomags))
  (if (not (== (Variables|Default|GetRifleTotalAmmo) 0))
    (if (< (Variables|Default|GetRifleTotalAmmo) 20)
      (Variables|Default|SetRifleCurrentAmmo (+ (Variables|Default|GetRifleTotalAmmo) _output))
      (Variables|Default|SetRifleTotalAmmo 0)
      (else
        (Variables|Default|SetRifleTotalAmmo (- (Variables|Default|GetRifleTotalAmmo) (- 20 _output)))
        (Variables|Default|SetRifleCurrentAmmo 20)))
    (CallFunction|UpdateAmmoMags)))

(fn RefillAmmo
  (params (RifleTotalAmmo :type Integer))
  (Variables|Default|SetRifleTotalAmmo RifleTotalAmmo))

(fn UpdateAmmoMags
  (bind _ammomags (Variables|Default|GetAmmoMags))
  (Utilities|Array|SetArrayElem _ammomags 0 (Variables|Default|GetRifleCurrentAmmo))
  (Utilities|Array|SetArrayElem _ammomags 1 (Variables|Default|GetRocketAmount))
  (Utilities|Array|SetArrayElem _ammomags 2 (Variables|Default|GetLaserAmount)))