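; BPC_Explosion is a component that gives its owning actor, stored as Bullet on BeginPlay, an explosion effect.
; Explode plays a fire sound and spawns BP_ExplodeParticles at the owner's location.
; It then fires the impulse of a radial component handed in through Init, if valid, and applies radial damage around the owner.
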(event EventBeginPlay
  (Variables|Default|SetBullet (Components|GetOwner)))

(event EventTick
  (params (DeltaSeconds :type Float%20%28single-precision%29)))

(fn Explode
  (bind _bullet (Variables|Default|GetBullet))
  (bind _returnvalue (Transformation|GetActorLocation _bullet))
  (Audio|PlaySoundatLocation "/Game/FPWeapon/Audio/FirstPersonTemplateWeaponFire02.FirstPersonTemplateWeaponFire02" _returnvalue "0, 0, 0" 1.0 1.0 0.0 0 0 0 0)
  (Game|SpawnActorfromClass "/Game/Tom/BluePrints/BP_ExplodeParticles.BP_ExplodeParticles_C" (Math|Transform|MakeTransform _returnvalue "0, 0, 0" "1.000000,1.000000,1.000000") "Undefined" "MultiplyWithRoot" 0 0)
  (Utilities|FlowControl|Sequence
    (:then_0
      (Utilities|IsValid (Variables|Default|GetRadialComp)
        (:Is%20Valid
          (Class|RadialForceComponent|FireImpulse (Variables|Default|GetRadialComp)))))
    (:then_1
      (Game|Damage|ApplyRadialDamage 1e+02 _returnvalue 1e+03 0 0 (Variables|Default|GetBullet) 0 false "ECC_Visibility"))))

(fn Init
  (params (RadialComp :type Radial%20Force%20Component%20Object%20Reference))
  (Variables|Default|SetRadialComp RadialComp))